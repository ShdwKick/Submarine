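; BP_Battery is an interactable energy pickup that recharges the player pawn and respawns after being collected.
; It starts hidden without collision, then appears after a spawn delay with a shine particle, whose template differs inside caves.
; Interaction below maximum energy passes the battery's energy to the pawn, plays a sound and hides the battery until the respawn delay ends.
; At full energy, it only shows a HUD notification.
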(event EventBeginPlay
  (bind _returnvalue (Transformation|GetActorLocation))
  (bind _battery (Variables|Default|GetBattery))
  (bind _battery_2 (Variables|Default|GetBattery))
  ;[0.1354 0.1354 0.1354 1 30] BeginPlay. Disable at first, spawn at delay
  (bind _returnvalue_2 (Effects|SpawnEmitteratLocation (select (Variables|Default|GetInCave) "/Game/VFX/Particles/Star_shineForCave.Star_shineForCave" "/Game/VFX/Particles/Star_shine1.Star_shine1") (Math|Vector|MakeVector (.x _returnvalue) (.y _returnvalue) (+ (.z _returnvalue) 5e+01)) "0, 0, 0" "2.000000,1.000000,1.000000" false "None" false))
  (Variables|Default|SetMyParticle _returnvalue_2)
  (Rendering|SetVisibility _battery_2 false true)
  (Collision|SetCollisionEnabled _battery_2 "NoCollision")
  (Utilities|FlowControl|Delay (Variables|Default|GetSpawnDelay))
  (Rendering|SetVisibility _battery true true)
  (Collision|SetCollisionEnabled _battery "QueryAndPhysics")
  (Components|Activation|Activate (Variables|Default|GetMyParticle) false))

(event EventInteraction
  (params (Short :type Boolean))
  (bind _battery (Variables|Default|GetBattery))
  (bind _battery_2 (Variables|Default|GetBattery))
  ;[0.1354 0.1354 0.1354 1 30] After interaction
  (bind _asbp_player_pawn (Utilities|Casting|CastToBP_PlayerPawn (Game|Player|GetPlayerPawn 0)))
  (if (< (Variables|/Script/Submarine.SubmarinePlayerPawnBase|GetPlayerEnergy _asbp_player_pawn) (Variables|/Script/Submarine.SubmarinePlayerPawnBase|GetMaxEnergyValue _asbp_player_pawn))
    ;;[0.1354 0.1354 0.1354 1 25] Collect and respawn
    (Default|CollectedBattery _asbp_player_pawn (Variables|Default|GetMyEnergy))
    (Audio|PlaySound2D "/Game/Sound/Other/Get_battery.Get_battery" 1.0 1.0 0.0 0 0)
    (Rendering|SetVisibility _battery false true)
    (Collision|SetCollisionEnabled _battery "NoCollision")
    (Components|Activation|Deactivate (Variables|Default|GetMyParticle))
    (Utilities|FlowControl|Delay (Variables|Default|GetRespawnDelay))
    (Rendering|SetVisibility _battery_2 true true)
    (Collision|SetCollisionEnabled _battery_2 "QueryAndPhysics")
    (Components|Activation|Activate (Variables|Default|GetMyParticle) false)
    (else
      (Default|Achievement/Notification (Variables|/Game/Blueprints/BP_PlayerPawn.BP_PlayerPawn_C|GetHUD _asbp_player_pawn) 0 "Батарея заполнена!" false 4.0))))

(fn ConstructionScript)