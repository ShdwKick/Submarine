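; BP_Chest is an interactable chest that grants resources and optionally an achievement message or end-game victory widget.
; Interaction runs once: it plays the open animation, pays out to BP_PlayerPawn, then after a delay fades out via a timeline-driven dynamic material.
; If respawnable, it schedules a replacement at a BP_ChestSpawnPoint before destroying itself.
; The random pick counts free points but indexes the full point list, so it can select an occupied one.
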(event Custom|AddEndGameWidget
  ;[0.1354 0.1354 0.1354 1 30] After interaction
  ;;[0.1354 0.1354 0.1354 1 25] Add end game widget
  (Utilities|FlowControl|Delay 3.0)
  (Audio|PlaySound2D "/Game/Sound/UI/victory.victory" 1.0 1.0 0.0 0 0)
  (bind _returnvalue (UserInterface|CreateWidget "/Game/Blueprints/OLD/UI/WB_EndGame.WB_EndGame_C"))
  (UserInterface|Viewport|AddtoViewport _returnvalue 0))

(event EventInteraction
  (params (Short :type Boolean))
  (bind _achievement (Variables|Default|GetAchievement))
  ;[0.1354 0.1354 0.1354 1 30] After interaction
  ;;[0.1354 0.1354 0.1354 1 25] To prevent multiple calls while animation is playing
  (Utilities|FlowControl|DoOnce false
    (:Completed
      ;;[0.1354 0.1354 0.1354 1 25] Play animation
      (Components|Animation|PlayAnimation (Variables|Default|GetSkeletalMesh) "/Game/Animations/Sunduk/Sunduk_Anim_Anim.Sunduk_Anim_Anim" false)
      ;;[0.1771 0.1771 0.1771] AddResourses
      (bind _asbp_player_pawn (Utilities|Casting|CastToBP_PlayerPawn (Game|Player|GetPlayerPawn 0)))
      (Default|AddResourses _asbp_player_pawn (Variables|Default|GetAddMap))
      ;;[0.1354 0.1354 0.1354 1 25] End game widget and add achievement if is valid
      (if (Variables|Default|GetEnd?)
        (CallFunction|AddEndGameWidget))
      (if (Utilities|IsValid _achievement)
        (Class|BPIGameInstance|AddAchievement(Message) (Game|GetGameInstance) _achievement))
      (Utilities|FlowControl|Delay 3.0)
      ;;[0.1354 0.1354 0.1354 1 25] Fade and destroy (and set new respawn point)
      (bind _fade (Timeline|ChestFadeOut Play)
        (:Update
          (Rendering|Material|SetScalarParameterValue (stale EventBeginPlay _returnvalue) "FadeOut" _fade :!class /Script/Engine.MaterialInstanceDynamic))
        (:Finished
          (if (Variables|Default|GetCanRespawn)
            (CallFunction|SetNewRespawnPoint))
          (Actor|DestroyActor))))))

(event EventBeginPlay
  ;[0.1354 0.1354 0.1354 1 25] BeginPlay Create Dynamic Material
  (bind _returnvalue (Rendering|Material|CreateDynamicMaterialInstance (Variables|Default|GetSkeletalMesh) 0 "/Game/Materials/M_Fade.M_Fade" "None" :!class /Script/Engine.PrimitiveComponent)))

(fn ConstructionScript)

(fn SetNewRespawnPoint
  (bind _outactors (Actor|GetAllActorsOfClass "/Game/Blueprints/Interactables/Chests/BP_ChestSpawnPoint.BP_ChestSpawnPoint_C"))
  (for (_array_element _array_index) _outactors
    (if (not (Default|CheckIsOccupied _array_element))
      (Utilities|Array|Add (LocalVariables|GetAvailablePoints) _array_index)))
  (Default|SpawnChestwithDelay (Utilities|Array|Get(acopy) _outactors (Math|Random|RandomInteger (Utilities|Array|Length (LocalVariables|GetAvailablePoints)))) (Variables|Default|GetAchievement) (Variables|Default|GetAddMap) (Variables|Default|GetRespawnDelay)))