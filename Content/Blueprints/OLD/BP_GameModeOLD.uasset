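; Older game mode Blueprint that shows the mouse cursor with Game and UI input and awards achievements through the Game Instance.
; On BeginPlay it binds to the player pawn's upgrade event and every BP_PathBlock's unlock event, and grants DeepDiving after a delay if not yet earned.
; Tag switches with DoOnce grant the matching achievements.
; A gate-based resource-count achievement remains as unreachable logic.
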(event Custom|UpgradeCalled
  (params (Tag :type Name))
  (bind _returnvalue (Game|GetGameInstance))
  ;[0.1354 0.1354 0.1354 1 30] Bind achievents
  ;;[0.1354 0.1354 0.1354] Upgrade achievements
  (switch name Tag
    (:Flashlight
      (Utilities|FlowControl|DoOnce false
        (:Completed
          (Class|BPIGameInstance|AddAchievement(Message) _returnvalue "/Game/Textures/2D/Achievements/MrLight.MrLight"))))
    (:SecondHand
      (Utilities|FlowControl|DoOnce false
        (:Completed
          (Class|BPIGameInstance|AddAchievement(Message) _returnvalue "/Game/Textures/2D/Achievements/ManyHands.ManyHands"))))
    (:BatteryLimit1
      (Utilities|FlowControl|DoOnce false
        (:Completed
          (Class|BPIGameInstance|AddAchievement(Message) _returnvalue "/Game/Textures/2D/Achievements/Charged.Charged"))))))

(event Custom|PathUnlocked
  (params (Tag :type Name))
  (bind _returnvalue (Game|GetGameInstance))
  ;[0.1354 0.1354 0.1354 1 30] Bind achievents
  ;;[0.1354 0.1354 0.1354] Pathblockers achievements
  (switch name Tag
    (:Flashlight
      (Utilities|FlowControl|DoOnce false
        (:Completed
          (Class|BPIGameInstance|AddAchievement(Message) _returnvalue "/Game/Textures/2D/Achievements/SecretPlace.SecretPlace"))))
    (:SecondHand
      (Utilities|FlowControl|DoOnce false
        (:Completed
          (Class|BPIGameInstance|AddAchievement(Message) _returnvalue "/Game/Textures/2D/Achievements/Ninja.Ninja"))))))

(event EventBeginPlay
  (bind _returnvalue (Game|GetGameInstance))
  ;[0.1354 0.1354 0.1354] Init
  (Utilities|FlowControl|Sequence
    (:then_0
      (bind _asbp_player_controller (Utilities|Casting|CastToBP_PlayerController (Game|GetPlayerController 0)))
      (Input|SetInputModeGameandUI _asbp_player_controller 0 "DoNotLock" true false)
      (Variables|/Script/Engine.PlayerController|SetbShowMouseCursor _asbp_player_controller true)
      ;[0.1354 0.1354 0.1354 1 30] Bind achievents
      (bind _asbp_player_pawn (Utilities|Casting|CastToBP_PlayerPawn (Game|Player|GetPlayerPawn 0)))
      (bind _output_get (Variables|Default|SetBPPawnRef _asbp_player_pawn))
      (EventDispatchers|BindEventtoUpgradeDone _output_get (delegate Custom|UpgradeCalled))
      (bind _outactors (Actor|GetAllActorsOfClass "/Game/Blueprints/PathBlockers/BP_PathBlock.BP_PathBlock_C"))
      (for _array_element _outactors
        (EventDispatchers|BindEventtoPathUnlocked _array_element (delegate Custom|PathUnlocked))))
    (:then_1
      (bind _achievenets (Class|BPIGameInstance|GetAchievements(Message) _returnvalue))
      (if (not (.Value (Utilities|Map|Find _achievenets "/Game/Textures/2D/Achievements/DeepDiving.DeepDiving")))
        (Utilities|FlowControl|Delay 3.0)
        (Class|BPIGameInstance|AddAchievement(Message) _returnvalue "/Game/Textures/2D/Achievements/DeepDiving.DeepDiving")))))

(fn ConstructionScript)