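; Player base actor, apparently an old version, that offers random quests and has upgradeable tiers.
; QuestEvent draws a quest number from a range widened by the pawn's Flashlight or SecondHand tags and fills the quest info widget.
; UpdateTier reads BaseTier tags from the pawn to toggle base component visibility and collision.
; BeginPlay is empty: tier setup, first timer, event binding, widget caching and HUD updates are disconnected.
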(event Custom|QuestEvent
  (bind _as_wb_quest_info (Variables|Default|GetAs%20WB%20Quest%20Info))
  ;[0.1354 0.1354 0.1354 1 30] Event new quest
  (Variables|Default|SetCurrentQuestNumber (Utilities|Select :Index (CallFunction|CheckEnabledLocations) :Option%200 (Math|Random|RandomIntegerinRange 1 3) :Option%201 (Math|Random|RandomIntegerinRange 1 8) :Option%202 (Math|Random|RandomIntegerinRange 1 13) :Option%203 0))
  (Widget|SetVisibility _as_wb_quest_info "Visible")
  (Default|ConstructQuest _as_wb_quest_info (Variables|Default|GetCurrentQuestNumber)))

(event Custom|PawnAcceptQuest
  ;[0.1354 0.1354 0.1354 1 30] Pawn Accept/Complete/Refuse Quest
  (Rendering|SetVisibility (Variables|Default|GetWidget%28BaseQuest%29) false false)
  (Rendering|SetVisibility (Variables|Default|GetWidget%28!%29) false false))

(event Custom|PawnCompleteQuest
  ;[0.1354 0.1354 0.1354 1 30] Pawn Accept/Complete/Refuse Quest
  (CallFunction|SetQuestTimer false))

(event Custom|PawnrefuseQuest
  ;[0.1354 0.1354 0.1354 1 30] Pawn Accept/Complete/Refuse Quest
  (Rendering|SetVisibility (Variables|Default|GetWidget%28!%29) false false)
  (Rendering|SetVisibility (Variables|Default|GetWidget%28BaseQuest%29) false false)
  (CallFunction|SetQuestTimer false))

(event Custom|SetQuestTimer
  (params (Initial :type Boolean))
  ;[0.1354 0.1354 0.1354 1 30] Set quest timer
  (bind _returnvalue (Utilities|Time|SetTimerbyEvent (EventDispatchers|CreateEvent :!event Custom|QuestEvent) (Variables|Default|GetQuestTimer%28sec%29) false (Math|Float|SelectFloat (Variables|Default|GetDelayBefore1stQuest) 0.0 Initial)))
  (Variables|Default|SetQuestTimer _returnvalue))

(event Custom|OpenQuestFromHUD
  ;[0.1354 0.1354 0.1354 1 30] OpenQuestFromHUD
  (UserInterface|Viewport|AddtoViewport (Variables|Default|GetAs%20WB%20Quest%20Info) 0)
  (Rendering|SetVisibility (Variables|Default|GetWidget%28BaseQuest%29) false false))

(event Custom|AttentionButtonClicked
  ;[0.1354 0.1354 0.1354 1 30] AttentionButtonClicked
  (Rendering|SetVisibility (Variables|Default|GetWidget%28BaseQuest%29) true false)
  (Widget|RemovefromParent (Variables|Default|GetAs%20WB%20Quest%20Info)))

(event EventBeginPlay
  ;[0.1354 0.1354 0.1354 1 30] Init
)

(fn ConstructionScript
  (Variables|Default|SetBaseComponentsArray (Utilities|Array|MakeArray (Variables|Default|GetBase) (Variables|Default|GetBase2) (Variables|Default|GetBase3) (Variables|Default|GetBase1))))

(fn UpdateTier
  (for _index (range (Variables|Default|GetCurrentBaseTier) (Variables|Default|GetMaxBaseTier))
    (if (not (< (Utilities|Array|FindItem (Variables|/Script/Engine.Actor|GetTags (Game|Player|GetPlayerPawn 0)) (Utilities|String|StringToName (Utilities|String|Append "BaseTier" (Utilities|String|ToString(Integer) _index)))) 0))
      (Variables|Default|SetCurrentBaseTier _index)))
  (for (_array_element _array_index) (Variables|Default|GetBaseComponentsArray)
    (if (<= _array_index (Variables|Default|GetCurrentBaseTier))
      (Rendering|SetVisibility _array_element true false)
      (Collision|SetCollisionEnabled _array_element "QueryAndPhysics")
      (else
        (Rendering|SetVisibility _array_element false false)
        (Collision|SetCollisionEnabled _array_element "NoCollision")))))

(fn CheckUpdateAvaliable
  (return (< (Variables|Default|GetCurrentBaseTier) (Variables|Default|GetMaxBaseTier))))

(fn GetUpgradeCost
  (return (Utilities|Select :Index (Variables|Default|GetCurrentBaseTier) :Option%200 (Variables|Default|GetUpgradeCostLvl1) :Option%201 (Variables|Default|GetUpgradeCostLvl2))))

(fn CheckEnabledLocations
  (bind _returnvalue (Game|Player|GetPlayerPawn 0))
  (if (Actor|ActorHasTag _returnvalue "Flashlight")
    (return 2)
    (elif (Actor|ActorHasTag _returnvalue "SecondHand")
      (return 1)
      (else
        (return 0)))))