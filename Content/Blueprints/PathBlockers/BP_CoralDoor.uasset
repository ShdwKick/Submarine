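; Coral path-blocker door that crumbles when its DestroyBlock event is called.
; The event turns off the Box collision and enables physics simulation on each of the many coral mesh pieces, while playing a staggered, layered 2D crush sound.
; Logic to record the door in the GameInstance's destroyed-door save list and destroy the actor is present but unconnected, so it never runs.
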(event EventDestroyBlock
  (Utilities|FlowControl|Sequence
    (:then_0
      (Collision|SetCollisionEnabled (Variables|Default|GetBox) "NoCollision")
      (for _array_element (Utilities|Array|MakeArray (Variables|Default|GetСorall_5_StaticMeshComponent0) (Variables|Default|GetСorall_13_StaticMeshComponent0) (Variables|Default|GetСorall_27_StaticMeshComponent0) (Variables|Default|GetСorall_25_StaticMeshComponent0) (Variables|Default|GetСorall_14_StaticMeshComponent0) (Variables|Default|GetСorall_20_StaticMeshComponent0) (Variables|Default|GetСorall_19_StaticMeshComponent0) (Variables|Default|GetСorall_18_StaticMeshComponent0) (Variables|Default|GetСorall_7_StaticMeshComponent0) (Variables|Default|GetСorall_8_StaticMeshComponent0) (Variables|Default|GetСorall_29_StaticMeshComponent0) (Variables|Default|GetСorall_32_StaticMeshComponent0) (Variables|Default|GetСorall_28_StaticMeshComponent0) (Variables|Default|GetСorall_17_StaticMeshComponent0) (Variables|Default|GetСorall_2_StaticMeshComponent0) (Variables|Default|GetСorall_21_StaticMeshComponent0) (Variables|Default|GetСorall_26_StaticMeshComponent0) (Variables|Default|GetСorall_4_StaticMeshComponent0) (Variables|Default|GetСorall_3_StaticMeshComponent0) (Variables|Default|GetСorall_23_StaticMeshComponent0) (Variables|Default|GetСorall_10_StaticMeshComponent0) (Variables|Default|GetСorall_65_StaticMeshComponent0) (Variables|Default|GetСorall_31_StaticMeshComponent0) (Variables|Default|GetСorall_24_StaticMeshComponent0) (Variables|Default|GetСorall_11_StaticMeshComponent0) (Variables|Default|GetСorall_9_StaticMeshComponent0) (Variables|Default|GetСorall_33_StaticMeshComponent0) (Variables|Default|GetСorall_12_StaticMeshComponent0) (Variables|Default|GetСorall_16_StaticMeshComponent0) (Variables|Default|GetСorall_15_StaticMeshComponent0) (Variables|Default|GetСorall_6_StaticMeshComponent0) (Variables|Default|GetСorall_41_StaticMeshComponent0) (Variables|Default|GetСorall_51_StaticMeshComponent0) (Variables|Default|GetСorall_36_StaticMeshComponent0) (Variables|Default|GetСorall_30_StaticMeshComponent0) (Variables|Default|GetСorall_46_StaticMeshComponent0) (Variables|Default|GetСorall_57_StaticMeshComponent0) (Variables|Default|GetСorall_63_StaticMeshComponent0) (Variables|Default|GetСorall_64_StaticMeshComponent0) (Variables|Default|GetСorall_56_StaticMeshComponent0) (Variables|Default|GetСorall_55_StaticMeshComponent0) (Variables|Default|GetСorall_50_StaticMeshComponent0) (Variables|Default|GetСorall_62_StaticMeshComponent0) (Variables|Default|GetСorall_61_StaticMeshComponent0) (Variables|Default|GetСorall_60_StaticMeshComponent0) (Variables|Default|GetСorall_59_StaticMeshComponent0) (Variables|Default|GetСorall_42_StaticMeshComponent0) (Variables|Default|GetСorall_54_StaticMeshComponent0) (Variables|Default|GetСorall_44_StaticMeshComponent0) (Variables|Default|GetСorall_45_StaticMeshComponent0) (Variables|Default|GetСorall_37_StaticMeshComponent0) (Variables|Default|GetСorall_38_StaticMeshComponent0) (Variables|Default|GetСorall_47_StaticMeshComponent0) (Variables|Default|GetСorall_35_StaticMeshComponent0) (Variables|Default|GetСorall_58_StaticMeshComponent0) (Variables|Default|GetСorall_34_StaticMeshComponent0) (Variables|Default|GetСorall_53_StaticMeshComponent0) (Variables|Default|GetСorall_52_StaticMeshComponent0) (Variables|Default|GetСorall_49_StaticMeshComponent0) (Variables|Default|GetСorall_40_StaticMeshComponent0) (Variables|Default|GetСorall_43_StaticMeshComponent0) (Variables|Default|GetСorall_39_StaticMeshComponent0) (Variables|Default|GetСorall_48_StaticMeshComponent0) (Variables|Default|GetСorall_22_StaticMeshComponent0))
        (Physics|SetSimulatePhysics _array_element true)
        (Utilities|FlowControl|Delay 5.0)))
    (:then_1
      (Audio|PlaySound2D "/Game/Sound/Other/coral_riff_crush.coral_riff_crush" 1.0 1.0 0.0 0 0)
      (Utilities|FlowControl|Delay 0.01)
      (Audio|PlaySound2D "/Game/Sound/Other/coral_riff_crush.coral_riff_crush" 1.0 1.0 0.0 0 0)
      (Utilities|FlowControl|Delay 0.1)
      (Audio|PlaySound2D "/Game/Sound/Other/coral_riff_crush.coral_riff_crush" 1.0 1.0 0.0 0 0))))

(fn ConstructionScript
  (|CallParentFunction))