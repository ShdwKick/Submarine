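; Base path blocker actor that bars the player until their pawn carries a required unlock tag.
; On BeginPlay it puts the needed-item icon into its WB_PathBlock_NeededItem widget.
; When the player pawn hits it, a matching tag triggers DestroyBlock, left empty for children to override, and a path-unlocked call.
; Without the tag, it shows the widget for two seconds; both outcomes show an emotion message on the pawn.
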(event Custom|DestroyBlock
  ;[1 1 1] Overrided in children
)

(event EventBeginPlay
  (bind _aswb_path_block_needed_item (Utilities|Casting|CastToWB_PathBlock_NeededItem (UserInterface|GetWidget (Variables|Default|GetWidget))))
  (Appearance|SetBrushfromTexture (Variables|/Game/Blueprints/PathBlockers/WB_PathBlock_NeededItem.WB_PathBlock_NeededItem_C|GetNeedenItem _aswb_path_block_needed_item) (Variables|Default|GetIconNeeded) false))

(event Collision|EventHit
  (params (MyComp :type Primitive%20Component%20Object%20Reference) (Other :type Actor%20Object%20Reference) (OtherComp :type Primitive%20Component%20Object%20Reference) (bSelfMoved :type Boolean) (HitLocation :type Vector :default "0, 0, 0") (HitNormal :type Vector :default "0, 0, 0") (NormalImpulse :type Vector :default "0, 0, 0") (Hit :type Hit%20Result%20Structure%20%28by%20ref%29))
  (bind _returnvalue (Game|Player|GetPlayerPawn 0))
  (bind _widget (Variables|Default|GetWidget))
  ;[1 1 1] Player tries to go through
  (if (== Other _returnvalue)
    (if (Actor|ActorHasTag _returnvalue (Variables|Default|GetPlayerTagForUnlock))
      (CallFunction|DestroyBlock)
      (Default|CallPathUnlocked (Variables|Default|GetPlayerTagForUnlock))
      (Class|BPIPlayer|ShowEmotion(Message) _returnvalue "NewEnumerator2" 1.5)
      (else
        (Rendering|SetVisibility _widget true false)
        (Class|BPIPlayer|ShowEmotion(Message) _returnvalue "NewEnumerator3" 1.5)
        (Utilities|FlowControl|Delay 2.0)
        (Rendering|SetVisibility _widget false false)))))

(fn ConstructionScript)