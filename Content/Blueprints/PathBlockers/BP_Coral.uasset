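; BP_Coral is a coral path blocker that breaks apart on interaction if the player pawn has the SecondHand tag, otherwise playing a not-enough-resources sound.
; Breaking plays a crush sound, calls CallDestroyed, disables the sphere collision and switches the stored meshes to physics simulation.
; After a delay it restores collision, returns each mesh to the transform cached at BeginPlay and becomes destructible again.
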(event EventInteraction
  (params (Short :type Boolean))
  (if (and (Actor|ActorHasTag (Game|Player|GetPlayerPawn 0) "SecondHand") (Variables|Default|GetCanDestroy))
    (Audio|PlaySound2D "/Game/Sound/Other/coral_riff_crush.coral_riff_crush" 1.0 1.0 0.0 0 0)
    (Default|CallDestroyed)
    (Variables|Default|SetCanDestroy false)
    (Collision|SetCollisionEnabled (Variables|Default|GetSphere) "NoCollision")
    (for _array_element (Variables|Default|GetMeshesArray)
      (Physics|SetSimulatePhysics _array_element true)
      (Collision|SetCollisionEnabled _array_element "PhysicsOnly"))
    (Utilities|FlowControl|Delay 25.0)
    (Collision|SetCollisionEnabled (Variables|Default|GetSphere) "QueryAndPhysics")
    (for (_array_element_2 _array_index) (Variables|Default|GetMeshesArray)
      (Physics|SetSimulatePhysics _array_element_2 false)
      (Transformation|SetWorldTransform _array_element_2 (Utilities|Array|Get(acopy) (Variables|Default|GetTransform) _array_index) false false)
      (Collision|SetCollisionEnabled _array_element_2 "QueryAndPhysics"))
    (Variables|Default|SetCanDestroy true)
    (else
      (Audio|PlaySound2D "/Game/Sound/UI/PopUps/not_enough_resources.not_enough_resources" 1.0 1.0 0.0 0 0))))

(event EventBeginPlay
  (for _array_element (Variables|Default|GetMeshesArray)
    (Utilities|Array|Add (Variables|Default|GetTransform) (Transformation|GetWorldTransform _array_element))))

(fn ConstructionScript
  (Utilities|Array|Add (Variables|Default|GetTags) (Variables|Default|GetTag)))