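; BP_Cave is a cave path blocker that switches the level to flashlight lighting inside.
; On BeginPlay it caches the level's directional light, then its in and out trigger overlaps hide or show that light and message the player pawn to enable or disable the flashlight.
; DestroyBlock, unless already done, calls DeletePlane on every BP_Cave in the world, which disables box collision, destroys the blocking plane and marks it done.
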(event OnComponentBeginOverlap(LightTriggerIn)
  (params (OverlappedComponent :type Primitive%20Component%20Object%20Reference) (OtherActor :type Actor%20Object%20Reference) (OtherComp :type Primitive%20Component%20Object%20Reference) (OtherBodyIndex :type Integer) (bFromSweep :type Boolean) (SweepResult :type Hit%20Result%20Structure%20%28by%20ref%29))
  (Rendering|SetVisibility (Variables|/Script/Engine.Light|GetLightComponent (Variables|Default|GetLightingComponent)) false false)
  (Class|BPIPlayer|SetFlashlightEnabled(Message) (Game|Player|GetPlayerPawn 0) true))

(event OnComponentBeginOverlap(LightTriggerOut)
  (params (OverlappedComponent :type Primitive%20Component%20Object%20Reference) (OtherActor :type Actor%20Object%20Reference) (OtherComp :type Primitive%20Component%20Object%20Reference) (OtherBodyIndex :type Integer) (bFromSweep :type Boolean) (SweepResult :type Hit%20Result%20Structure%20%28by%20ref%29))
  (Rendering|SetVisibility (Variables|/Script/Engine.Light|GetLightComponent (Variables|Default|GetLightingComponent)) true false)
  (Class|BPIPlayer|SetFlashlightEnabled(Message) (Game|Player|GetPlayerPawn 0) false))

(event Custom|DeletePlane
  (Collision|SetCollisionEnabled (Variables|Default|GetBox) "NoCollision")
  (Components|DestroyComponent (Variables|Default|GetPlane1))
  (Variables|Default|SetDone true))

(event EventBeginPlay
  (|CallParentFunction)
  (bind _returnvalue (Actor|GetActorOfClass "/Script/Engine.DirectionalLight"))
  (Variables|Default|SetLightingComponent _returnvalue))

(event Collision|EventActorBeginOverlap
  (params (OtherActor :type Actor%20Object%20Reference)))

(event EventTick
  (params (DeltaSeconds :type Float%20%28single-precision%29)))

(event EventDestroyBlock
  (if (not (Variables|Default|GetDone))
    (bind _outactors (Actor|GetAllActorsOfClass "BP_Cave_C"))
    (for _array_element _outactors
      (CallFunction|DeletePlane _array_element))))

(fn ConstructionScript
  (|CallParentFunction))