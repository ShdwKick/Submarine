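; Octopus path blocker that the player feeds to clear the way and earn a chest.
; On hit or overlap, Eat checks the pawn's three food-stage tags from highest to lowest and sets the hunger widget's fill.
; Each stage reacts once with an emotion, eating call and temporary socketed food mesh; the first also grants an achievement.
; The final stage plays the rise animation, disables box collision, spawns BP_Chest and destroys the octopus.
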(event EventBeginPlay
  (|CallParentFunction) ; This node is disabled and will not be called.\nDrag off pins to build functionality.
)

(event EventTick
  (params (DeltaSeconds :type Float%20%28single-precision%29)))

(event Collision|EventActorBeginOverlap
  (params (OtherActor :type Actor%20Object%20Reference))
  (if (== OtherActor (Game|Player|GetPlayerPawn 0))
    (bind _aswb_octopus_widget (Utilities|Casting|CastToWB_OctopusWidget (UserInterface|GetWidget (Variables|Default|GetHunger))))
    (Utilities|Eat 1.0 "HaveOctFood3" 0 _aswb_octopus_widget
      (:Has
        (Variables|Default|SetDone true)
        (Utilities|FlowControl|DoOnce false
          (:Completed
            _)))
      (:DontHave
        (Utilities|Eat 0.65 "HaveOctFood2" 0 _aswb_octopus_widget
          (:Has
            (Utilities|FlowControl|DoOnce false
              (:Completed
                _)))
          (:DontHave
            (Utilities|Eat 0.35 "HaveOctFood1" 0 _aswb_octopus_widget
              (:Has
                (Utilities|FlowControl|DoOnce false
                  (:Completed
                    _))))))))
    (Class|BPIPlayer|ShowEmotion(Message) (Game|Player|GetPlayerPawn 0) "NewEnumerator2" 1.5)
    (Default|CallEating)
    (Utilities|FlowControl|Sequence
      (:then_0
        (Utilities|FlowControl|DoOnce false
          (:Completed
            (Class|BPIGameInstance|AddAchievement(Message) (Game|GetGameInstance) "/Game/Textures/2D/Achievements/Octopus.Octopus"))))
      (:then_1
        (Utilities|FlowControl|Delay 1.0)
        (bind _returnvalue (AddComponent|AddStaticMeshComponent true))
        (Transformation|AttachComponentToComponent _returnvalue (Variables|Default|GetOctopus_Skelet) "Food" "KeepRelative" "KeepRelative" "KeepRelative" true)
        (Utilities|FlowControl|Delay 1.0)
        (Components|DestroyComponent _returnvalue))
      (:then_2
        (if (Variables|Default|GetDone)
          (Utilities|FlowControl|Delay 2.0)
          (Components|Animation|PlayAnimation (Variables|Default|GetOctopus_Skelet) "/Game/Animations/Osminog/AS_Octopus_Up.AS_Octopus_Up" false)
          (Rendering|SetVisibility (Variables|Default|GetHunger) false false)
          (Collision|SetCollisionEnabled (Variables|Default|GetBox) "NoCollision")
          (Utilities|FlowControl|Delay 0.5)
          (Game|SpawnActorfromClass "/Game/Blueprints/Interactables/Chests/BP_Chest.BP_Chest_C" (Math|Transform|MakeTransform (+ (.location (Transformation|GetActorTransform)) "0.000000,50.000000,0.000000") "0.000000,90.000000,0.000000" "3.000000,3.000000,3.000000") "Undefined" "MultiplyWithRoot" 0 "/Game/Textures/2D/Achievements/Captain.Captain" true 0)
          (Utilities|FlowControl|Delay 5.0)
          (Actor|DestroyActor))))))

(event Collision|EventHit
  (params (MyComp :type Primitive%20Component%20Object%20Reference) (Other :type Actor%20Object%20Reference) (OtherComp :type Primitive%20Component%20Object%20Reference) (bSelfMoved :type Boolean) (HitLocation :type Vector :default "0, 0, 0") (HitNormal :type Vector :default "0, 0, 0") (NormalImpulse :type Vector :default "0, 0, 0") (Hit :type Hit%20Result%20Structure%20%28by%20ref%29))
  (if (== Other (Game|Player|GetPlayerPawn 0))
    (bind _aswb_octopus_widget (Utilities|Casting|CastToWB_OctopusWidget (UserInterface|GetWidget (Variables|Default|GetHunger))))
    (Utilities|Eat 1.0 "HaveOctFood3" 0 _aswb_octopus_widget
      (:Has
        (Variables|Default|SetDone true)
        (Utilities|FlowControl|DoOnce false
          (:Completed
            _)))
      (:DontHave
        (Utilities|Eat 0.65 "HaveOctFood2" 0 _aswb_octopus_widget
          (:Has
            (Utilities|FlowControl|DoOnce false
              (:Completed
                _)))
          (:DontHave
            (Utilities|Eat 0.35 "HaveOctFood1" 0 _aswb_octopus_widget
              (:Has
                (Utilities|FlowControl|DoOnce false
                  (:Completed
                    _))))))))
    (Class|BPIPlayer|ShowEmotion(Message) (Game|Player|GetPlayerPawn 0) "NewEnumerator2" 1.5)
    (Default|CallEating)
    (Utilities|FlowControl|Sequence
      (:then_0
        (Utilities|FlowControl|DoOnce false
          (:Completed
            (Class|BPIGameInstance|AddAchievement(Message) (Game|GetGameInstance) "/Game/Textures/2D/Achievements/Octopus.Octopus"))))
      (:then_1
        (Utilities|FlowControl|Delay 1.0)
        (bind _returnvalue (AddComponent|AddStaticMeshComponent true))
        (Transformation|AttachComponentToComponent _returnvalue (Variables|Default|GetOctopus_Skelet) "Food" "KeepRelative" "KeepRelative" "KeepRelative" true)
        (Utilities|FlowControl|Delay 1.0)
        (Components|DestroyComponent _returnvalue))
      (:then_2
        (if (Variables|Default|GetDone)
          (Utilities|FlowControl|Delay 2.0)
          (Components|Animation|PlayAnimation (Variables|Default|GetOctopus_Skelet) "/Game/Animations/Osminog/AS_Octopus_Up.AS_Octopus_Up" false)
          (Rendering|SetVisibility (Variables|Default|GetHunger) false false)
          (Collision|SetCollisionEnabled (Variables|Default|GetBox) "NoCollision")
          (Utilities|FlowControl|Delay 0.5)
          (Game|SpawnActorfromClass "/Game/Blueprints/Interactables/Chests/BP_Chest.BP_Chest_C" (Math|Transform|MakeTransform (+ (.location (Transformation|GetActorTransform)) "0.000000,50.000000,0.000000") "0.000000,90.000000,0.000000" "3.000000,3.000000,3.000000") "Undefined" "MultiplyWithRoot" 0 "/Game/Textures/2D/Achievements/Captain.Captain" true 0)
          (Utilities|FlowControl|Delay 5.0)
          (Actor|DestroyActor))))))

(fn ConstructionScript
  (|CallParentFunction))