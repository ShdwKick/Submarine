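; BP_GarbageSpawner keeps a BP_Garbage actor spawned at its own transform, respawning it after it is destroyed.
; It spawns one on BeginPlay and binds to that garbage's OnDestroyed event to start a timer of RespawnTime.
; When the timer fires, TryRespawnGarbage rolls a weighted chance (RespawnChance) to spawn a new piece, or restarts the timer to try again.
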(event Custom|GarbageDestroyed
  (params (DestroyedActor :type Actor%20Object%20Reference))
  (Utilities|Time|SetTimerbyFunctionName 0 "TryRespawnGarbage" (Variables|Default|GetRespawnTime)))

(event Custom|SpawnNewGarbage
  (bind _returnvalue (Game|SpawnActorfromClass "/Game/Blueprints/NewMechanics/Garbage/BP_Garbage.BP_Garbage_C" (Transformation|GetActorTransform) "Undefined" "MultiplyWithRoot" 0 0))
  (Game|BindEventtoOnDestroyed _returnvalue (delegate Custom|GarbageDestroyed)))

(event EventBeginPlay
  (CallFunction|SpawnNewGarbage))

(fn ConstructionScript)

(fn TryRespawnGarbage
  (if (Math|Random|RandomBoolwithWeight (Variables|Default|GetRespawnChance))
    (CallFunction|SpawnNewGarbage)
    (else
      (Utilities|Time|SetTimerbyFunctionName 0 "TryRespawnGarbage" (Variables|Default|GetRespawnTime)))))