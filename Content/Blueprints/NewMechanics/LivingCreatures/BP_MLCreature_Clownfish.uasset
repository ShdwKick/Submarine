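; Clownfish variant of a living creature, made up of a group of ten fish components that turn to face the direction the actor moves.
; A fast looping timer started at BeginPlay, used instead of Tick, smoothly interpolates each fish's world rotation toward the velocity direction, with a yaw offset.
; The construction script passes the fish components to AddMaterialsToArray.
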(event Custom|RotateActorByMoveDirection
  (if (> (Math|Vector|VectorLength (Transformation|GetVelocity)) 0.0)
    (for _array_element (Variables|Default|GetArray)
      (Transformation|SetWorldRotation _array_element (Math|Interpolation|RInterpTo (Transformation|GetWorldRotation _array_element) (Math|Rotator|MakeRotator (.Roll (Math|Rotator|BreakRotator (Math|Rotator|FindLookatRotation (Transformation|GetWorldLocation _array_element) (+ (Transformation|GetWorldLocation _array_element) (* (Math|Vector|Normalize (Transformation|GetVelocity)) 1.5e+02))))) (.Pitch (Math|Rotator|BreakRotator (Math|Rotator|FindLookatRotation (Transformation|GetWorldLocation _array_element) (+ (Transformation|GetWorldLocation _array_element) (* (Math|Vector|Normalize (Transformation|GetVelocity)) 1.5e+02))))) (- (.Yaw (Math|Rotator|BreakRotator (Math|Rotator|FindLookatRotation (Transformation|GetWorldLocation _array_element) (+ (Transformation|GetWorldLocation _array_element) (* (Math|Vector|Normalize (Transformation|GetVelocity)) 1.5e+02))))) 9e+01)) (Utilities|Time|GetWorldDeltaSeconds) 3.0) true false))))

(event EventBeginPlay
  (|CallParentFunction)
  (Variables|Default|SetArray (Utilities|Array|MakeArray (Variables|Default|GetFish3) (Variables|Default|GetFish4) (Variables|Default|GetFish5) (Variables|Default|GetFish2) (Variables|Default|GetFish1) (Variables|Default|GetFish10) (Variables|Default|GetFish9) (Variables|Default|GetFish8) (Variables|Default|GetFish6) (Variables|Default|GetFish7)))
  (Utilities|Time|SetTimerbyEvent (delegate Custom|RotateActorByMoveDirection) 0.01 true))

(event Collision|EventActorBeginOverlap
  (params (OtherActor :type Actor%20Object%20Reference)))

(event EventTick
  (params (DeltaSeconds :type Float%20%28single-precision%29))
  (|CallParentFunction DeltaSeconds) ; This node is disabled and will not be called.\nDrag off pins to build functionality.
)

(fn ConstructionScript
  (|CallParentFunction)
  (CallFunction|AddMaterialstoArray (Utilities|Array|MakeArray (Variables|Default|GetFish8) (Variables|Default|GetFish4) (Variables|Default|GetFish5) (Variables|Default|GetFish7) (Variables|Default|GetFish6) (Variables|Default|GetFish3) (Variables|Default|GetFish9) (Variables|Default|GetFish10) (Variables|Default|GetFish2) (Variables|Default|GetFish1))))