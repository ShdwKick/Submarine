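; Dolphin creature Blueprint that turns its skeletal mesh to face the direction it is moving.
; On BeginPlay it runs the parent logic and starts a fast looping timer that stands in for the disabled Tick.
; While velocity is non-zero, the timer smoothly interpolates the mesh's world rotation toward the velocity direction, with a yaw offset of minus 90 degrees and sweep enabled.
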(event Custom|CustomEvent
  (if (> (Math|Vector|VectorLength (Transformation|GetVelocity)) 0.0)
    (for _array_element (Variables|Default|GetArray)
      (Transformation|SetWorldRotation _array_element (Math|Interpolation|RInterpTo (Transformation|GetWorldRotation _array_element) (Math|Rotator|MakeRotator (.Roll (Math|Rotator|BreakRotator (Math|Rotator|FindLookatRotation (Transformation|GetWorldLocation _array_element) (+ (Transformation|GetWorldLocation _array_element) (* (Math|Vector|Normalize (Transformation|GetVelocity)) 1.5e+02))))) (.Pitch (Math|Rotator|BreakRotator (Math|Rotator|FindLookatRotation (Transformation|GetWorldLocation _array_element) (+ (Transformation|GetWorldLocation _array_element) (* (Math|Vector|Normalize (Transformation|GetVelocity)) 1.5e+02))))) (- (.Yaw (Math|Rotator|BreakRotator (Math|Rotator|FindLookatRotation (Transformation|GetWorldLocation _array_element) (+ (Transformation|GetWorldLocation _array_element) (* (Math|Vector|Normalize (Transformation|GetVelocity)) 1.5e+02))))) 9e+01)) (Utilities|Time|GetWorldDeltaSeconds) 4.0) true false))))

(event EventBeginPlay
  (|CallParentFunction)
  (Variables|Default|SetArray (Utilities|Array|MakeArray (Variables|Default|GetSkeletalMesh)))
  (Utilities|Time|SetTimerbyEvent (delegate Custom|CustomEvent) 0.01 true))

(event Collision|EventActorBeginOverlap
  (params (OtherActor :type Actor%20Object%20Reference)))

(event EventTick
  (params (DeltaSeconds :type Float%20%28single-precision%29))
  (|CallParentFunction DeltaSeconds) ; This node is disabled and will not be called.\nDrag off pins to build functionality.
)

(fn ConstructionScript
  (|CallParentFunction))