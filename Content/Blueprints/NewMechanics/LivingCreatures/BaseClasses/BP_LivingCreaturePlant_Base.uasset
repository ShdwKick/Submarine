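; Base Blueprint for living plant creatures, with debug display of their health.
; BeginPlay caches the debug health widget, Tick writes current Health to it, and HealthBigChange recolors its text across three states.
; A helper collects dynamic material instances from supplied skeletal components into Materials, but is not called here.
; The per-state BaseColor texture swap on those materials is left disconnected, so state changes leave them untouched.
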(event EventBeginPlay
  (|CallParentFunction)
  (bind _aswbp_debug_health (Utilities|Casting|CastToWBP_DebugHealth (UserInterface|GetWidget (Variables|Default|GetDebugHealth))))
  (Variables|Default|SetAs%20WBP%20Debug%20Health _aswbp_debug_health))

(event EventHealthBigChange
  (params (OldState :type Integer) (NewState :type Integer))
  (Variables|/Script/UMG.TextBlock|SetColorAndOpacity (Variables|/Game/Blueprints/NewMechanics/LivingCreatures/BaseClasses/WBP_DebugHealth.WBP_DebugHealth_C|GetHealth (Variables|Default|GetAs%20WBP%20Debug%20Health)) (Utilities|Struct|MakeSlateColor (Utilities|Select :Index NewState :Option%200 "(R=0.208333,G=0.000000,B=0.018368,A=1.000000)" :Option%201 "(R=1.000000,G=0.665931,B=0.143740,A=1.000000)" :Option%202 "(R=0.000000,G=1.000000,B=0.070008,A=1.000000)")))
  (if (!= OldState NewState)
    (for _array_element (Variables|Default|GetMaterials)
      _)))

(event EventTick
  (params (DeltaSeconds :type Float%20%28single-precision%29))
  (Rendering|Components|TextRender|SetText (Variables|/Game/Blueprints/NewMechanics/LivingCreatures/BaseClasses/WBP_DebugHealth.WBP_DebugHealth_C|GetHealth (Variables|Default|GetAs%20WBP%20Debug%20Health)) (Utilities|Text|ToText(Float) (Variables|Default|GetHealth) "HalfToEven")))

(fn ConstructionScript)

(fn AddMaterialstoArray
  (params (SkeletalComponents :type Array%20of%20Skeletal%20Mesh%20Component%20Object%20References))
  (for _array_element SkeletalComponents
    (bind _returnvalue (Rendering|Material|CreateDynamicMaterialInstance _array_element 0 (Rendering|Material|GetMaterial _array_element 0) "None" :!class /Script/Engine.PrimitiveComponent))
    (Utilities|Array|Add (Variables|Default|GetMaterials) _returnvalue)))