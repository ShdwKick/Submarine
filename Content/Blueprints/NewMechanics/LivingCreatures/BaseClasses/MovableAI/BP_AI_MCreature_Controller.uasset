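; AI controller for movable living creatures that starts the BT_MovableCreature behavior tree on BeginPlay.
; Perception updates feed the blackboard: actors implementing BPI_Player set BB_Player when sensed and clear it when lost.
; Other actors tagged Food fill BB_Food and FoodObject only while no valid food is held, so the creature keeps that target even after losing sight of it.
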(event OnTargetPerceptionUpdated(AIPerception)
  (params (Actor :type Actor%20Object%20Reference) (Stimulus :type AI%20Stimulus%20Structure))
  (bind _bsuccessfullysensed (Utilities|Struct|BreakAIStimulus Stimulus))
  (bind _returnvalue (AI|GetBlackboard 0))
  (bind _returnvalue_2 (Utilities|SelectObject Actor 0 _bsuccessfullysensed))
  (Utilities|IsValid Actor
    (:Is%20Valid
      (if (Utilities|DoesObjectImplementInterface Actor "/Game/Blueprints/BPI_Player.BPI_Player_C")
        (AI|Components|Blackboard|SetValueasObject _returnvalue (Utilities|Name|MakeLiteralName "BB_Player") (Utilities|SelectObject Actor 0 _bsuccessfullysensed))
        (elif (Actor|ActorHasTag Actor "Food")
          (Utilities|IsValid (Variables|Default|GetFoodObject)
            (:Is%20Not%20Valid
              (AI|Components|Blackboard|SetValueasObject _returnvalue (Utilities|Name|MakeLiteralName "BB_Food") _returnvalue_2)
              (Variables|Default|SetFoodObject _returnvalue_2))))))))

(event EventBeginPlay
  (AI|RunBehaviorTree "/Game/Blueprints/NewMechanics/LivingCreatures/BaseClasses/MovableAI/BT_MovableCreature.BT_MovableCreature"))

(fn ConstructionScript)