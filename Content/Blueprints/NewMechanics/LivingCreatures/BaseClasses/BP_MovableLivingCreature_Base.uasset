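; Base Blueprint for AI living creatures that wander, eat food objects and can become friendly to or tamed by the player.
; It feeds blackboard keys for a behaviour tree, choosing wander points near a local spot or, after a periodic random migration roll, across a wider start area.
; Sphere overlaps register food and player; feeding near the player raises a decaying count that sets friendliness.
; A debug widget shows health, migration and feeding.
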(event OnComponentBeginOverlap(SphereCollision)
  (params (OverlappedComponent :type Primitive%20Component%20Object%20Reference) (OtherActor :type Actor%20Object%20Reference) (OtherComp :type Primitive%20Component%20Object%20Reference) (OtherBodyIndex :type Integer) (bFromSweep :type Boolean) (SweepResult :type Hit%20Result%20Structure%20%28by%20ref%29))
  (bind _self self)
  (bind _returnvalue (AI|GetAIController _self))
  (bind _returnvalue_2 (AI|GetBlackboard _returnvalue))
  ;[1 1 1] interaction
  (bind _asbp_feeding_object (Utilities|Casting|CastToBP_FeedingObject OtherActor)
    (:then
      (if (Class|BlackboardComponent|IsVectorValueSet (AI|GetBlackboard (AI|GetAIController self)) (Utilities|Name|MakeLiteralName "BB_Food"))
        (Utilities|Array|AddUnique (Variables|Default|GetAnotherFeedingObjects) _asbp_feeding_object)
        (else
          (AI|Components|Blackboard|SetValueasVector _returnvalue_2 (Utilities|Name|MakeLiteralName "BB_Food") (Math|Vector|MakeVector (.X (Math|Vector|BreakVector (Transformation|GetActorLocation _asbp_feeding_object))) (.Y (Math|Vector|BreakVector (Transformation|GetActorLocation _asbp_feeding_object))) (.z (Transformation|GetActorLocation))))
          (AI|Components|Blackboard|SetValueasObject _returnvalue_2 (Utilities|Name|MakeLiteralName "BB_FoodObject") _asbp_feeding_object))))
    (:CastFailed
      (bind _asbp_player_pawn (Utilities|Casting|CastToBP_PlayerPawn OtherActor))
      (Variables|Default|SetOverlappedPlayer _asbp_player_pawn)
      (AI|Components|Blackboard|SetValueasObject (AI|GetBlackboard (AI|GetAIController self)) (Utilities|Name|MakeLiteralName "BB_Player") _asbp_player_pawn)
      (AI|Components|Blackboard|SetValueasBool (AI|GetBlackboard (AI|GetAIController self)) (Utilities|Name|MakeLiteralName "BB_IsPlayerFriendly") (>= (Variables|Food|GetFeedingCount) 2)))))

(event OnComponentEndOverlap(SphereCollision)
  (params (OverlappedComponent :type Primitive%20Component%20Object%20Reference) (OtherActor :type Actor%20Object%20Reference) (OtherComp :type Primitive%20Component%20Object%20Reference) (OtherBodyIndex :type Integer))
  (bind _targetlocationtimer (Variables|Default|GetTargetLocationTimer))
  ;[1 1 1] interaction
  (Utilities|Casting|CastToBP_PlayerPawn OtherActor)
  (AI|Components|Blackboard|ClearValue (AI|GetBlackboard (AI|GetAIController self)) (Utilities|Name|MakeLiteralName "BB_Player"))
  (Variables|Default|SetOverlappedPlayer 0)
  (Utilities|Time|PauseTimerbyHandle _targetlocationtimer)
  (Utilities|Time|ClearandInvalidateTimerbyHandle _targetlocationtimer))

(event Custom|RotateActorByMoveDirection
  (bind _returnvalue (Transformation|GetVelocity))
  (bind _returnvalue_2 (Transformation|GetActorLocation))
  (bind _returnvalue_3 (Math|Vector|Normalize _returnvalue))
  (bind _returnvalue_4 (* _returnvalue_3 1.5e+02))
  (bind _returnvalue_5 (+ _returnvalue_2 _returnvalue_4))
  (bind _returnvalue_6 (Math|Rotator|FindLookatRotation _returnvalue_2 _returnvalue_5))
  (bind (_roll _pitch _yaw) (Math|Rotator|BreakRotator _returnvalue_6))
  ;[0.1771 0.1771 0.1771] Rotation
  (Transformation|SetActorRotation (Math|Rotator|MakeRotator _roll _pitch (- _yaw 9e+01))))

(event Custom|FoodWasEaten
  (bind _self self)
  (bind _returnvalue (AI|GetAIController _self))
  (bind _returnvalue_2 (AI|GetBlackboard _returnvalue))
  ;[0.1771 0.1771 0.1771 1 30] Food consumed
  (AI|Components|Blackboard|ClearValue _returnvalue_2 (Utilities|Name|MakeLiteralName "BB_Food"))
  (AI|Components|Blackboard|ClearValue _returnvalue_2 (Utilities|Name|MakeLiteralName "BB_FoodObject"))
  (Class|MovableLivingCreature|FoodConsumed)
  (CallFunction|FindNextFood)
  (Utilities|IsValid (AI|Components|Blackboard|GetValueasObject (AI|GetBlackboard (AI|GetAIController self)) (Utilities|Name|MakeLiteralName "BB_FoodObject"))
    (:Is%20Valid
      _)
    (:Is%20Not%20Valid
      (CallFunction|GetNextPointtoMove)))
  (Math|Integer|IncrementInt (Variables|Food|GetFeedingCount)
    (:%20%20
      (if (> (Utilities|Array|Length (Collision|GetOverlappingActors "/Game/Blueprints/BP_PlayerPawn.BP_PlayerPawn_C" :!class /Script/Engine.Actor)) 0)
        (Rendering|Components|TextRender|SetText (Variables|/Game/Blueprints/NewMechanics/LivingCreatures/BaseClasses/WBP_DebugHealth.WBP_DebugHealth_C|GetTextBlock_Feeding (Variables|Default|GetAs%20WBP%20Debug%20Health)) (Utilities|Text|FormatText "Feed: {food}" (Variables|Food|GetFeedingCount)))
        (bind _returnvalue_3 (Utilities|Time|SetTimerbyEvent (delegate Custom|DecreaseFood) (Variables|Food|GetFoodConumingForgetTime) true))
        (Variables|Food|SetFoodConsumingTimer _returnvalue_3)))))

(event Custom|GetNextPointToMove
  (bind _startpoint (Variables|Default|GetStartPoint))
  (bind _localstartpoint (Variables|Default|GetLocalStartPoint))
  (bind (_randomlocation _returnvalue) (AI|Navigation|GetRandomReachablePointinRadius _localstartpoint 5e+02 0 0))
  (bind (_randomlocation_2 _returnvalue_2) (AI|Navigation|GetRandomReachablePointinRadius _startpoint 1.8e+03 0 0))
  ;[1 1 1] movement
  (if (Variables|Default|GetIsCanMigrate)
    (if _returnvalue_2
      (AI|Components|Blackboard|SetValueasVector (AI|GetBlackboard (AI|GetAIController self)) (Utilities|Name|MakeLiteralName "BB_MigrationPoint") (Math|Vector|MakeVector (.x _randomlocation_2) (.y _randomlocation_2) (.z (Transformation|GetActorLocation)))))
    (elif _returnvalue
      (AI|Components|Blackboard|SetValueasVector (AI|GetBlackboard (AI|GetAIController self)) (Utilities|Name|MakeLiteralName "BB_MigrationPoint") (Math|Vector|MakeVector (.x _randomlocation) (.y _randomlocation) (.z (Transformation|GetActorLocation)))))))

(event Custom|CheckIsCanMigrate
  (bind _output_get (Variables|Default|SetIsCanMigrate (Math|Random|RandomBoolwithWeight 0.05)))
  (if _output_get
    _
    (else
      (Variables|Default|SetLocalStartPoint (Transformation|GetActorLocation))))
  (Rendering|Components|TextRender|SetText (Variables|/Game/Blueprints/NewMechanics/LivingCreatures/BaseClasses/WBP_DebugHealth.WBP_DebugHealth_C|GetTextBlock_Migration (Variables|Default|GetAs%20WBP%20Debug%20Health)) (Utilities|Text|FormatText "Mig: {status}" _output_get)))

(event Custom|DecreaseFood
  (bind _feedingcount (Variables|Food|GetFeedingCount))
  (bind _foodconsumingtimer (Variables|Food|GetFoodConsumingTimer))
  ;[0.1771 0.1771 0.1771 1 30] Food consumed
  (Rendering|Components|TextRender|SetText (Variables|/Game/Blueprints/NewMechanics/LivingCreatures/BaseClasses/WBP_DebugHealth.WBP_DebugHealth_C|GetTextBlock_Feeding (Variables|Default|GetAs%20WBP%20Debug%20Health)) (Utilities|Text|FormatText "Feed: {food}" (Variables|Food|GetFeedingCount)))
  (Math|Integer|DecrementInt _feedingcount
    (:%20%20
      (AI|Components|Blackboard|SetValueasBool (AI|GetBlackboard (AI|GetAIController self)) (Utilities|Name|MakeLiteralName "BB_IsPlayerFriendly") (>= (Variables|Food|GetFeedingCount) 2))
      (if (== _feedingcount 0)
        (Utilities|Time|PauseTimerbyHandle _foodconsumingtimer)
        (Utilities|Time|ClearandInvalidateTimerbyHandle _foodconsumingtimer)))))

(event Custom|CalculateTargetLocation
  ;[1 1 1] interaction
  (if (>= (Variables|Food|GetFeedingCount) 2)
    (AI|Components|Blackboard|SetValueasVector (AI|GetBlackboard (AI|GetAIController self)) (Utilities|Name|MakeLiteralName "BB_TargetLocation") (Transformation|GetActorLocation (Variables|Default|GetOverlappedPlayer)))
    (Development|PrintString "Hello")))

(event EventBeginPlay
  (bind _returnvalue (Transformation|GetActorLocation))
  ;[0.1771 0.1771 0.1771 1 30] Init
  (bind _aswbp_debug_health (Utilities|Casting|CastToWBP_DebugHealth (UserInterface|GetWidget (Variables|Default|GetDebugHealth))))
  (Variables|Default|SetAs%20WBP%20Debug%20Health _aswbp_debug_health)
  (Utilities|FlowControl|Delay 0.1)
  (Components|Sphere|SetSphereRadius (Variables|Default|GetMigrationDetectDebug) (.MigratePointsDetectRadius (Utilities|Struct|BreakLivingCreatureInfo (Variables|Default|GetCreatureInfo))) true)
  (Variables|Default|SetStartPoint _returnvalue)
  (Variables|Default|SetLocalStartPoint _returnvalue)
  (AI|Components|Blackboard|SetValueasVector (AI|GetBlackboard (AI|GetAIController self)) (Utilities|Name|MakeLiteralName "BB_MigrationPoint") (Transformation|GetActorLocation))
  (AI|Components|Blackboard|ClearValue (AI|GetBlackboard (AI|GetAIController self)) (Utilities|Name|MakeLiteralName "BB_Food"))
  (CallFunction|GetNextPointtoMove)
  (Utilities|Time|SetTimerbyEvent (delegate Custom|CheckIsCanMigrate) 72.0 true 2.0)
  (bind _output_get (Variables|Default|SetIsCanMigrate (Math|Random|RandomBoolwithWeight 0.05)))
  (if _output_get
    _
    (else
      (Variables|Default|SetLocalStartPoint (Transformation|GetActorLocation))))
  (Rendering|Components|TextRender|SetText (Variables|/Game/Blueprints/NewMechanics/LivingCreatures/BaseClasses/WBP_DebugHealth.WBP_DebugHealth_C|GetTextBlock_Migration (Variables|Default|GetAs%20WBP%20Debug%20Health)) (Utilities|Text|FormatText "Mig: {status}" _output_get)))

(event EventHealthBigChange
  (params (OldState :type Integer) (NewState :type Integer))
  ;[0.1771 0.1771 0.1771 1 30] Health Big Change
  (Variables|/Script/UMG.TextBlock|SetColorAndOpacity (Variables|/Game/Blueprints/NewMechanics/LivingCreatures/BaseClasses/WBP_DebugHealth.WBP_DebugHealth_C|GetHealth (Variables|Default|GetAs%20WBP%20Debug%20Health)) (Utilities|Struct|MakeSlateColor (Utilities|Select :Index NewState :Option%200 "(R=0.208333,G=0.000000,B=0.018368,A=1.000000)" :Option%201 "(R=1.000000,G=0.665931,B=0.143740,A=1.000000)" :Option%202 "(R=0.000000,G=1.000000,B=0.070008,A=1.000000)")))
  (if (!= OldState NewState)
    (for _array_element (Variables|Default|GetMaterials)
      _)))

(event EventTick
  (params (DeltaSeconds :type Float%20%28single-precision%29))
  ;[0.1771 0.1771 0.1771 1 30] Tick (ShowHealth)
)

(event EventEventTamed
  (bind _returnvalue (Transformation|GetActorLocation))
  ;[0.1771 0.1771 0.1771 1 30] Tamed
  (Niagara|SpawnSystematLocation "/Game/sA_Megapack_v1/sA_PickupSet_1/Fx/NiagaraSystems/NS_Healing_1.NS_Healing_1" _returnvalue)
  (Audio|PlaySoundatLocation "/Game/Sound/UI/Achive2.Achive2" _returnvalue "0, 0, 0" 1.0 1.0 0.0 0 0 0 0)
  (AI|Components|Blackboard|SetValueasBool (AI|GetBlackboard (AI|GetAIController self)) (Utilities|Name|MakeLiteralName "BB_Tamed") true))

(event EventFoodDetected
  (params (FoodActor :type Feeding%20Object%20Object%20Reference))
  ;[0.1771 0.1771 0.1771 1 30] Food Detected
)

(event EventMigrationInitiatedBP
  (params (MigrationPoint :type Actor%20Object%20Reference))
  ;[0.1771 0.1771 0.1771 1 30] Migration init
  (AI|Components|Blackboard|SetValueasObject (AI|GetBlackboard (AI|GetAIController self)) (Utilities|Name|MakeLiteralName "BB_MigrationPoint") MigrationPoint))

(event EventEventPlayerDetected
  (params (Player :type Actor%20Object%20Reference))
  ;[0.1771 0.1771 0.1771 1 30] Player detection
)

(event EventPlayerLost
  ;[0.1771 0.1771 0.1771 1 30] Player detection
)

(fn ConstructionScript
  (|CallParentFunction))

(fn AddMaterialstoArray
  (params (SkeletalComponents :type Array%20of%20Skeletal%20Mesh%20Component%20Object%20References))
  (for _array_element SkeletalComponents
    (bind _returnvalue (Rendering|Material|CreateDynamicMaterialInstance _array_element 0 (Rendering|Material|GetMaterial _array_element 0) "None" :!class /Script/Engine.PrimitiveComponent))
    (Utilities|Array|Add (Variables|Default|GetMaterials) _returnvalue)))

(fn GetAllMigrationPoints
  (bind _outactors (Collision|SphereOverlapActors (Transformation|GetActorLocation) (Utilities|Struct|BreakLivingCreatureInfo (Variables|Default|GetCreatureInfo)) (Utilities|Array|MakeArray "ObjectTypeQuery2" "ObjectTypeQuery1" "ObjectTypeQuery6") "/Game/Blueprints/NewMechanics/LivingCreatures/BaseClasses/BP_MigrationPoint.BP_MigrationPoint_C"))
  (return _outactors))

(fn DoesPouintHaveBetterInfluence
  (params (Point :type Vector))
  (Collision|SphereOverlapActors Point (Components|Sphere|GetScaledSphereRadius (Variables|Default|GetSphereCollision)) (Utilities|Array|MakeArray "ObjectTypeQuery2" "ObjectTypeQuery1" "ObjectTypeQuery6") 0))

(fn FindNextFood
  (bind _self self)
  (bind _anotherfeedingobjects (Variables|Default|GetAnotherFeedingObjects))
  (bind _returnvalue (AI|GetAIController _self))
  (bind _output (Utilities|Array|Get(acopy) _anotherfeedingobjects))
  (bind _returnvalue_2 (Transformation|GetActorLocation _output))
  (bind _returnvalue_3 (AI|GetBlackboard _returnvalue))
  (bind (_x _y) (Math|Vector|BreakVector _returnvalue_2))
  (if (> (Utilities|Array|Length (Variables|Default|GetAnotherFeedingObjects)) 0)
    (if (< (Math|Vector|Distance(Vector) (Transformation|GetActorLocation _output) (Transformation|GetActorLocation)) 6e+02)
      (AI|Components|Blackboard|SetValueasVector _returnvalue_3 (Utilities|Name|MakeLiteralName "BB_Food") (Math|Vector|MakeVector _x _y (.z (Transformation|GetActorLocation))))
      (AI|Components|Blackboard|SetValueasObject _returnvalue_3 (Utilities|Name|MakeLiteralName "BB_FoodObject") _output))
    (Utilities|Array|RemoveItem (Variables|Default|GetAnotherFeedingObjects) _output)))