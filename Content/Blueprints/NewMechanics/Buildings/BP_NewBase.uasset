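; BP_NewBase is an upgradable base building that saves the game when the player pawn overlaps its sphere.
; BeginPlay caches the submarine game mode, which the overlap event calls to save.
; UpgradeBase resizes the sphere and cascades through levels one to three, so each level also enables the lower levels' meshes.
; EnableBaseElement makes a part visible and gives it blocking collision.
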(event OnComponentBeginOverlap(SphereCollision)
  (params (OverlappedComponent :type Primitive%20Component%20Object%20Reference) (OtherActor :type Actor%20Object%20Reference) (OtherComp :type Primitive%20Component%20Object%20Reference) (OtherBodyIndex :type Integer) (bFromSweep :type Boolean) (SweepResult :type Hit%20Result%20Structure%20%28by%20ref%29))
  (Utilities|Casting|CastToBP_PlayerPawn OtherActor)
  (bind _submarine_game_mode (Variables|Default|GetSubmarine%20Game%20Mode)
    (:then
      (Default|SaveGame _submarine_game_mode))
    (:else)))

(event Custom|UpgradeBase
  (params (NewLvl :type Integer) (NewRadius :type Float%20%28double-precision%29))
  (Components|Sphere|SetSphereRadius (Variables|Default|GetSphereCollision) NewRadius true)
  (switch int NewLvl
    (:1
      _)
    (:2
      (CallFunction|EnableBaseElement (Variables|Default|GetBase3) :!label _label))
    (:3
      (CallFunction|EnableBaseElement (Variables|Default|GetBase2))
      (goto _label)))
  (CallFunction|EnableBaseElement (Variables|Default|GetBase1)))

(event EventBeginPlay
  (bind _asbp_submarine_game_mode (Utilities|Casting|CastToBP_SubmarineGameMode (Game|GetGameMode)))
  (Variables|Default|SetSubmarine%20Game%20Mode _asbp_submarine_game_mode))

(fn ConstructionScript)

(fn EnableBaseElement
  (params (Component :type Primitive%20Component%20Object%20Reference))
  (Rendering|SetVisibility Component true false)
  (Collision|SetCollisionProfileName Component "BlockAllCollision" true :!class /Script/Engine.PrimitiveComponent))