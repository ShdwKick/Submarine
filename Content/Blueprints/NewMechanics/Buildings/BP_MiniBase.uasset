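; BP_MiniBase is a purchasable mini-base site that the player swaps for a built BP_NewMiniBase by paying resources.
; Its widget receives the cost on BeginPlay, and sphere overlap shows or hides the player HUD's build widget, with debug prints and a box.
; InitializeBuy checks and spends the player's resources, then spawns the new base in place and destroys this actor.
; Inventory, widget-update and upgrade events are empty, with their old logic left disconnected.
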(event OnComponentBeginOverlap(SphereCollision)
  (params (OverlappedComponent :type Primitive%20Component%20Object%20Reference) (OtherActor :type Actor%20Object%20Reference) (OtherComp :type Primitive%20Component%20Object%20Reference) (OtherBodyIndex :type Integer) (bFromSweep :type Boolean) (SweepResult :type Hit%20Result%20Structure%20%28by%20ref%29))
  (bind _asbp_player_pawn (Utilities|Casting|CastToBP_PlayerPawn OtherActor))
  (bind _output_get (Variables|Default|SetPlayer _asbp_player_pawn))
  (Development|PrintString (Utilities|String|ToString(Text) (Utilities|Text|FormatText "is valid {is}" (Utilities|IsValid (Variables|/Game/Blueprints/BP_PlayerPawn.BP_PlayerPawn_C|GetNewHUD _output_get)))))
  (Default|GetHUD _output_get)
  (Development|PrintString (Utilities|String|ToString(Text) (Utilities|Text|FormatText "hud is valid {is}" (Utilities|IsValid 0))))
  (Default|ShowBuildWidget (Variables|/Game/Blueprints/BP_PlayerPawn.BP_PlayerPawn_C|GetNewHUD _output_get) (Variables|Default|GetResources) self)
  (Rendering|Debug|DrawDebugBox (Transformation|GetActorLocation) "75.000000,75.000000,75.000000" "(R=0.073681,G=1.000000,B=0.000000,A=1.000000)" "0, 0, 0" 2.0 5.0))

(event OnComponentEndOverlap(SphereCollision)
  (params (OverlappedComponent :type Primitive%20Component%20Object%20Reference) (OtherActor :type Actor%20Object%20Reference) (OtherComp :type Primitive%20Component%20Object%20Reference) (OtherBodyIndex :type Integer))
  (bind _asbp_player_pawn (Utilities|Casting|CastToBP_PlayerPawn OtherActor))
  (Default|HideBuildWidget (Variables|/Game/Blueprints/BP_PlayerPawn.BP_PlayerPawn_C|GetNewHUD _asbp_player_pawn))
  (Variables|Default|SetPlayer 0))

(event Custom|UpgradeMiniBase
  (params (NewRadius :type Float%20%28double-precision%29)))

(event Custom|InventoryUpdate
  (params (ItemType :type EItem%20Enum :default "Bronze") (Count :type Integer) (Add? :type Boolean)))

(event Custom|InitializeBuy
  (bind _player (Variables|Default|GetPlayer))
  (bind _resources (Variables|Default|GetResources))
  (Utilities|IsValid _player
    (:Is%20Valid
      (bind _returnvalue (Class|SubmarinePlayerPawnBase|CheckInventoryHaveResourses _player _resources))
      (if _returnvalue
        (bind _purchasedone (Default|PurchasebyResourses _player _resources))
        (if _purchasedone
          (Game|SpawnActorfromClass "/Game/Blueprints/NewMechanics/Buildings/BP_NewMiniBase.BP_NewMiniBase_C" (Transformation|GetActorTransform) "Undefined" "MultiplyWithRoot" 0 0)
          (Actor|DestroyActor))))))

(event EventBeginPlay
  (|CallParentFunction)
  (bind _aswbp_buy_mini_base_widget (Utilities|Casting|CastToWBP_BuyMiniBaseWidget (UserInterface|GetWidget (Variables|Default|GetWidget))))
  (Variables|/Game/Blueprints/NewMechanics/Widgets/MiniBase/WBP_BuyMiniBaseWidget.WBP_BuyMiniBaseWidget_C|SetResources _aswbp_buy_mini_base_widget (Variables|Default|GetResources)))

(event EventUpdateWidget
  (params (bHide :type Boolean)))

(fn ConstructionScript)