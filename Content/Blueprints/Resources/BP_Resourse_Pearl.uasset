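; BP_Resourse_Pearl is a pearl resource actor that highlights itself when the player pawn overlaps it.
; Overlap begin applies M_OverlayHighlight as an overlay material on the skeletal mesh, and overlap end clears it for that pawn.
; Both overlap events call the parent's begin-overlap handler, including the end event.
; The construction script only calls its parent, and BeginPlay is disabled.
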(event EventBeginPlay
  (|CallParentFunction) ; This node is disabled and will not be called.\nDrag off pins to build functionality.
)

(event Collision|EventActorBeginOverlap
  (params (OtherActor :type Actor%20Object%20Reference))
  (|CallParentFunction 0)
  (if (== OtherActor (Game|Player|GetPlayerPawn 0))
    (Rendering|Material|SetOverlayMaterial (Variables|Default|GetSkeletalMesh) "/Game/Materials/M_OverlayHighlight.M_OverlayHighlight" :!class /Script/Engine.MeshComponent)))

(event Collision|EventActorEndOverlap
  (params (OtherActor :type Actor%20Object%20Reference))
  (|CallParentFunction OtherActor)
  (if (== OtherActor (Game|Player|GetPlayerPawn 0))
    (Rendering|Material|SetOverlayMaterial (Variables|Default|GetSkeletalMesh) 0 :!class /Script/Engine.MeshComponent)))

(fn ConstructionScript
  (|CallParentFunction))