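; Player controller that links the player pawn to the HUD widget and enables the mouse cursor with Game and UI input.
; On BeginPlay it binds to the pawn's on-base change event, which shows or hides the HUD's base-related buttons.
; A NewLivingCreature event passes an icon to the HUD's living creature button.
; Cursor switching for Spawner-tagged actors and a debug language toggle are present but disconnected, so Tick does nothing.
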(event Custom|ShowHide_BaseRelatedButtons
  (params (IsOnBase :type Boolean))
  ;[0.1771 0.1771 0.1771] Initiaction
  (bind _aswb_hudnew (Utilities|Casting|CastToWB_HUDNew (Variables|Default|GetHUD)))
  (if IsOnBase
    (Default|ShowBaseRelatedButtons _aswb_hudnew)
    (else
      (Default|HideBaseRelatedButtons _aswb_hudnew))))

(event Custom|NewLivingCreature
  (params (Icon :type Texture%202D%20Object%20Reference))
  ;[0.1771 0.1771 0.1771] New Living Creature
  (bind _aswb_hudnew (Utilities|Casting|CastToWB_HUDNew (Variables|Default|GetHUD)))
  (Default|SetNewAnimal (Variables|/Game/Blueprints/NewMechanics/Widgets/WB_HUDNew.WB_HUDNew_C|GetLivingCratureButton _aswb_hudnew) Icon))

(event EventTick
  (params (DeltaSeconds :type Float%20%28single-precision%29))
  ;[0.3177 0.1145 0.09866] Change mouse cursor
)

(event EventBeginPlay
  ;[0.1771 0.1771 0.1771] Initiaction
  (|CallParentFunction)
  (Input|SetInputModeGameandUI self 0 "LockOnCapture" false false)
  (Variables|Default|SetbShowMouseCursor true)
  (bind _asbp_player_pawn (Utilities|Casting|CastToBP_PlayerPawn (Game|Player|GetPlayerPawn 0)))
  (EventDispatchers|BindEventtoIsonBaseChanged _asbp_player_pawn (delegate Custom|ShowHide_BaseRelatedButtons)))

(event Input|KeyboardEvents|L
  (params (Key :type Key%20Structure :default "None"))
  ;[0.3177 0.1145 0.09866] For debug
)

(fn ConstructionScript)