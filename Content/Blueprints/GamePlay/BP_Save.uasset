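; BP_Save is a save game object that stores master and music volume settings, plus temporary copies of both.
; Each setter updates its value and immediately saves the object to the "Settings" slot.
; Each getter reloads that slot, casts it to BP_Save and returns one value.
; SetMusicVolume fills the other Settings field with the previous music volume rather than preserving master volume.
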(event Custom|SaveMasterVolume
  (params (Value :type Float%20%28double-precision%29))
  (Variables|Default|SetSettings (Utilities|Struct|MakeSettings Value (.musicvolume (Variables|Default|GetSettings))))
  (SaveGame|SaveGametoSlot self "Settings"))

(event Custom|SetMusicVolume
  (params (Value :type Float%20%28double-precision%29))
  (Variables|Default|SetSettings (Utilities|Struct|MakeSettings (.musicvolume (Variables|Default|GetSettings)) Value))
  (SaveGame|SaveGametoSlot self "Settings"))

(event Custom|SaveTempMusicVolume
  (params (Value :type Float%20%28double-precision%29))
  (Variables|Default|SetTempMusicVolume Value)
  (SaveGame|SaveGametoSlot self "Settings"))

(event Custom|SaveTempMasterVolume
  (params (Value :type Float%20%28double-precision%29))
  (Variables|Default|SetTempMasterVolume Value)
  (SaveGame|SaveGametoSlot self "Settings"))

(fn LoadTempMusicVolume
  (bind _returnvalue (SaveGame|LoadGamefromSlot "Settings"))
  (bind _asbp_save (Utilities|Casting|CastToBP_Save _returnvalue))
  (return (Variables|BP_Save_C|GetTempMusicVolume _asbp_save)))

(fn LoadTempMasterVolume
  (bind _returnvalue (SaveGame|LoadGamefromSlot "Settings"))
  (bind _asbp_save (Utilities|Casting|CastToBP_Save _returnvalue))
  (return (Variables|BP_Save_C|GetTempMasterVolume _asbp_save)))

(fn LoadMasterVolume
  (bind _returnvalue (SaveGame|LoadGamefromSlot "Settings"))
  (bind _asbp_save (Utilities|Casting|CastToBP_Save _returnvalue))
  (return (.mastervolume (Variables|BP_Save_C|GetSettings _asbp_save))))

(fn LoadMusicVolume
  (bind _returnvalue (SaveGame|LoadGamefromSlot "Settings"))
  (bind _asbp_save (Utilities|Casting|CastToBP_Save _returnvalue))
  (return (.musicvolume (Variables|BP_Save_C|GetSettings _asbp_save))))