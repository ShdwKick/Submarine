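; Blueprint function library that fills a parent widget with cost entries for resources or currencies.
; Each function clears the parent, then adds a padded WB_CostResourse with amount and icon per cost key.
; Resource icons come from DT_ResoursesData, while currency icons are selected inline, with all reputation types sharing one.
; The player pawn's inventory or wallet is checked to show a Done mark on affordable entries.
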(fn ConstructCostResourses
  (params (Cost :type Map%20of%20EItem%20Enums%20to%20Integers :default "Bronze") (ParentWidget :type Panel%20Widget%20Object%20Reference))
  (Widget|Panel|ClearChildren ParentWidget)
  (bind _keys (Utilities|Map|Keys Cost))
  (bind _array_element (Utilities|Array|ForEachLoopwithBreak _keys)
    (:LoopBody
      (bind _returnvalue (Utilities|GetDataTableRow "/Game/Blueprints/Resources/DT_ResoursesData.DT_ResoursesData" (Utilities|Select :Index _array_element :Bronze "Bronze" :Gold "Gold" :Platinum "Platinum" :BlueCrystall "BlueCrystal" :GreenCrystall "GreenCrystal" :RedCrystall "RedCrystal" :Chemicals "Chemicals" :Food "Food"))
        (:then
          (bind _returnvalue_2 (UserInterface|CreateWidget "/Game/Blueprints/NewMechanics/Widgets/StoreUpgrades/WB_CostResourse.WB_CostResourse_C" 0 (Utilities|Text|ToText(Integer) (.Value (Utilities|Map|Find Cost _array_element))) (.Icon (Utilities|Struct|BreakResourseData _returnvalue))))
          (bind _inventory (Class|BPIPlayer|NewGetInventory(Message) (Game|Player|GetPlayerPawn 0)))
          (if (< (.Value (Utilities|Map|Find _inventory _array_element)) (.Value (Utilities|Map|Find Cost _array_element)))
            _
            (else
              (Widget|SetVisibility (Variables|/Game/Blueprints/NewMechanics/Widgets/StoreUpgrades/WB_CostResourse.WB_CostResourse_C|GetDone _returnvalue_2) "Visible")))
          (Layout|BorderSlot|SetPadding _returnvalue_2 (Utilities|Struct|MakeMargin 4.0 0.0 4.0 0.0) :!class /Script/UMG.UserWidget)
          (Widget|Panel|AddChild ParentWidget _returnvalue_2))))
    (:Completed
      (return))))

(fn ConstructCostCurrency
  (params (Cost :type Map%20of%20ECurrency%20Enums%20to%20Integers :default "Money") (ParentWidget :type Panel%20Widget%20Object%20Reference))
  (Widget|Panel|ClearChildren ParentWidget)
  (bind _keys (Utilities|Map|Keys Cost))
  (bind _array_element (Utilities|Array|ForEachLoopwithBreak _keys)
    (:LoopBody
      (bind _returnvalue (UserInterface|CreateWidget "/Game/Blueprints/NewMechanics/Widgets/StoreUpgrades/WB_CostResourse.WB_CostResourse_C" 0 (Utilities|Text|ToText(Integer) (.Value (Utilities|Map|Find Cost _array_element))) (Utilities|Select :Index _array_element :Money "/Game/Blueprints/NewMechanics/Widgets/2D/HUD/Dollar.Dollar" :ScienceRep "/Game/Blueprints/NewMechanics/Widgets/2D/HUD/Reputation.Reputation" :EcologyRep "/Game/Blueprints/NewMechanics/Widgets/2D/HUD/Reputation.Reputation" :BusinessRep "/Game/Blueprints/NewMechanics/Widgets/2D/HUD/Reputation.Reputation" :GarbageRep "/Game/Blueprints/NewMechanics/Widgets/2D/HUD/Reputation.Reputation")))
      (bind _wallet (Class|BPIPlayer|NewGetWallet(Message) (Game|Player|GetPlayerPawn 0)))
      (if (< (.Value (Utilities|Map|Find _wallet _array_element)) (.Value (Utilities|Map|Find Cost _array_element)))
        _
        (else
          (Widget|SetVisibility (Variables|/Game/Blueprints/NewMechanics/Widgets/StoreUpgrades/WB_CostResourse.WB_CostResourse_C|GetDone _returnvalue) "Visible")))
      (Layout|BorderSlot|SetPadding _returnvalue (Utilities|Struct|MakeMargin 4.0 0.0 4.0 0.0) :!class /Script/UMG.UserWidget)
      (Widget|Panel|AddChild ParentWidget _returnvalue))
    (:Completed
      (return))))